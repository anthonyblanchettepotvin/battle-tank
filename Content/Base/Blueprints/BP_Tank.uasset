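; Player-controllable tank Blueprint that drives on two tracks, aims its camera and fires.
; On BeginPlay it hands the barrel and turret to AimingComponent and both tracks to MovementComponent.
; Throttle and per-track axes become forward and turn intents on MovementComponent, while Fire calls AimingComponent.
; Aim axes rotate the azimuth gimbal and spring arm, scaled by delta time, rather than moving the turret directly.
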(event EventBeginPlay
  (Class|TankAimingComponent|Initialize (Variables|Default|GetAimingComponent) (Variables|Default|GetBarrel) (Variables|Default|GetTurret))
  (Class|TankMovementComponent|Initialize (Variables|Default|GetMovementComponent) (Variables|Default|GetTrackLeft) (Variables|Default|GetTrackRight)))

(event Collision|EventActorBeginOverlap
  (params (OtherActor :type Actor%20Object%20Reference)))

(event EventTick
  (params (DeltaSeconds :type Float%20%28single-precision%29)))

(event Input|ActionEvents|InputActionFire
  (params (Key :type Key%20Structure :default "None"))
  (:Pressed
    (Class|TankAimingComponent|Fire (Variables|Default|GetAimingComponent))))

(event Input|AxisEvents|InputAxisAimAzimuth
  (params (AxisValue :type Float%20%28single-precision%29))
  (Transformation|AddLocalRotation (Variables|Default|GetAzimuthGimbal) (Math|Rotator|MakeRotator 0.0 0.0 (* AxisValue (Utilities|Time|GetWorldDeltaSeconds) 1e+02)) false false))

(event Input|AxisEvents|InputAxisAimElevation
  (params (AxisValue :type Float%20%28single-precision%29))
  (Transformation|AddLocalRotation (Variables|Default|GetSpringArm) (Math|Rotator|MakeRotator 0.0 (* AxisValue (Utilities|Time|GetWorldDeltaSeconds) 1e+02) 0.0) false false))

(event Input|AxisEvents|InputAxisLeftTrackThrottle
  (params (AxisValue :type Float%20%28single-precision%29))
  (Class|TankMovementComponent|IntendMoveForward (Variables|Default|GetMovementComponent) (/ (+ (stale Input|AxisEvents|InputAxisRightTrackThrottle AxisValue) AxisValue) 2.0)))

(event Input|AxisEvents|InputAxisRightTrackThrottle
  (params (AxisValue :type Float%20%28single-precision%29))
  (Class|TankMovementComponent|IntendTurnRight (Variables|Default|GetMovementComponent) (- AxisValue (stale Input|AxisEvents|InputAxisLeftTrackThrottle AxisValue))))

(event Input|AxisEvents|InputAxisThrolleForward
  (params (AxisValue :type Float%20%28single-precision%29))
  (Class|TankMovementComponent|IntendMoveForward (Variables|Default|GetMovementComponent) AxisValue))

(event Input|AxisEvents|InputAxisThrolleRight
  (params (AxisValue :type Float%20%28single-precision%29))
  (Class|TankMovementComponent|IntendTurnRight (Variables|Default|GetMovementComponent) AxisValue))

(fn ConstructionScript)